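; Player character for a twin-stick flying shooter, with movement, aiming, health, a play timer, HUD widgets and a pause menu.
; Aim input rotates the controller and starts looping Fire once; the timer-clearing nodes are unwired.
; Space triggers an overdrive speed boost, afterburner and seven-point volley when MaxStamina reaches 100, and release restores speed.
; Stamina regen is ineffective because its only call passes UsingStamina as true, and polarity switching is disconnected.
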(event `Key|SpaceBar`
  (params (Key :type "Key Structure"))
  ;[1 1 1] Stamina Recharge System
  (:`Pressed`
    (`self.Regen Stamina` true)))

(event `Regen Stamina`
  (params (`Using Stamina` :type Boolean))
  ;[1 1 1] Regen Stamina
  (if (and (not `Using Stamina`) (< (`self.Stamina`) (`self.Max Stamina`)))
    (bind _output_get (set `self.Stamina Regen Delay Time` (+ (`GameplayStatics.GetWorldDeltaSeconds`) (`self.Stamina Regen Delay Time`))))
    (if (>= _output_get (`self.Stamina Regen Delay Time`))
      (set `self.Stamina` (+ (`self.Stamina`) (* (`GameplayStatics.GetWorldDeltaSeconds`) (`self.Stamina Regen Amount`))))
      (if (< (`self.Stamina`) (`self.Max Stamina`))
        (set `self.Max Stamina` 50.0)
        (else
          (set `self.Max Stamina` 50.0))))))

(event `self.ReceiveTick`
  (params (DeltaSeconds :type "Float (single-precision)"))
  ;[1 1 1] Timer
  (`|ExecutionSequence`
    (:`then_1`
      (`KismetSystemLibrary.Delay` 1.0)
      (set `self.TimeSec` (+ (`self.TimeSec`) 1))
      (if (> (`self.TimeSec`) 59)
        (set `self.TimeMin` (+ (`self.TimeMin`) 1))
        (set `self.TimeSec` 0)))))

(event `Key|SpaceBar`
  (params (Key :type "Key Structure"))
  (bind _charactermovement (`self.CharacterMovement`))
  ;[1 1 1] Overdrive
  (:`Pressed`
    (if (>= (`self.Max Stamina`) 100.0)
      (set `CharacterMovementComponent.MaxFlySpeed` 1800.0 _charactermovement)
      (`|ExecutionSequence`
        (:`then_0`
          (bind _output_get (set `self.AfterBurnerOD` (`self.AfterBurnerOD`)))
          (`ActorComponent.Activate` _output_get true)
          (`KismetSystemLibrary.Delay` 2.0)
          (`ActorComponent.Deactivate` _output_get))
        (:`then_1`
          ;[1 1 1] Multi-Shot
          (`|ExecutionSequence`
            (:`then_0`
              (`|SpawnActorFromClass` "/Game/Blueprints/Projectile.Projectile_C" (`SceneComponent.K2_GetComponentToWorld` (`self.OD 1`)) "Undefined" "OverrideRootScale" null null))
            (:`then_1`
              (`|SpawnActorFromClass` "/Game/Blueprints/Projectile.Projectile_C" (`SceneComponent.K2_GetComponentToWorld` (`self.OD 2`)) "Undefined" "OverrideRootScale" null null))
            (:`then_2`
              (`|SpawnActorFromClass` "/Game/Blueprints/Projectile.Projectile_C" (`SceneComponent.K2_GetComponentToWorld` (`self.OD 3`)) "Undefined" "OverrideRootScale" null null))
            (:`then_3`
              (`|SpawnActorFromClass` "/Game/Blueprints/Projectile.Projectile_C" (`SceneComponent.K2_GetComponentToWorld` (`self.OD 4`)) "Undefined" "OverrideRootScale" null null))
            (:`then_4`
              (`|SpawnActorFromClass` "/Game/Blueprints/Projectile.Projectile_C" (`SceneComponent.K2_GetComponentToWorld` (`self.OD 5`)) "Undefined" "OverrideRootScale" null null))
            (:`then_5`
              (`|SpawnActorFromClass` "/Game/Blueprints/Projectile.Projectile_C" (`SceneComponent.K2_GetComponentToWorld` (`self.OD 6`)) "Undefined" "OverrideRootScale" null null))
            (:`then_6`
              (`|SpawnActorFromClass` "/Game/Blueprints/Projectile.Projectile_C" (`SceneComponent.K2_GetComponentToWorld` (`self.OD 7`)) "Undefined" "OverrideRootScale" null null)))))))
  (:`Released`
    (set `CharacterMovementComponent.MaxFlySpeed` 1200.0 _charactermovement)
    (bind _output_get_2 (set `self.AfterBurner` (`self.AfterBurner`)))
    (`ActorComponent.Activate` _output_get_2 true)))

(event `self.ReceiveBeginPlay`
  ;[1 1 1] Shows the Health Bar on the viewport
  (`|ExecutionSequence`
    (:`then_0`
      ;[1 1 1] Timer: UI
      (bind _returnvalue (`|CreateWidget` "/Game/Blueprints/Timer.Timer_C"))
      (bind _output_get (set `self.Timer` _returnvalue))
      (`UserWidget.AddToViewport` _output_get 0))
    (:`then_1`
      (bind _returnvalue_2 (`|CreateWidget` "/Game/Blueprints/HealthBar.HealthBar_C"))
      (`UserWidget.AddToViewport` _returnvalue_2 0))
    (:`then_2`)))

(event `Key|E`
  (params (Key :type "Key Structure"))
  ;[1 1 1] Polarity Switch / Link Broken since it doesn't work
)

(event `/Game/Blueprints/Damageable.Take Damage`
  (params (Damage :type "Float (single-precision)"))
  ;[1 1 1] Player Health
  (bind _output_get (set `self.Health` (- (`self.Health`) Damage)))
  (`KismetSystemLibrary.PrintString` (`KismetStringLibrary.Conv_DoubleToString` _output_get) false)
  (if (<= (`self.Health`) 0.0)
    (`self.K2_DestroyActor`)))

(event `Fire`
  ;[1 1 1] Shooting
  (`|SpawnActorFromClass` "/Game/Blueprints/Projectile.Projectile_C" (`SceneComponent.K2_GetComponentToWorld` (`self.Spawn`)) "Undefined" "OverrideRootScale" null null)
  (`GameplayStatics.SpawnSound2D` "/Engine/VREditor/Sounds/UI/Laser_Pull.Laser_Pull" 0.2 1.0 0.0 null))

(event `InputAxis|MoveRight`
  (params (AxisValue :type "Float (single-precision)"))
  ;[1 1 1] Movement
  (`self.AddMovementInput` (0.0 1.0 0.0) AxisValue))

(event `InputAxis|Aim Up`
  (params (AxisValue :type "Float (single-precision)"))
  ;[1 1 1] Rotation
  (bind _returnvalue (`KismetMathLibrary.MakeVector` AxisValue (stale `InputAxis|Aim Right` AxisValue)))
  (if (> (`KismetMathLibrary.VSize` _returnvalue) 0.25) :!label _label
    (`Controller.SetControlRotation` (`self.GetController`) (`KismetMathLibrary.Conv_VectorToRotator` _returnvalue))
    ;[1 1 1] Pull/Release Trigger
    (`KismetSystemLibrary.Delay` 0.0)
    (`/Engine/EditorBlueprintResources/StandardMacros.DoOnce` false
      (:`Completed`
        (`self.Fire`)
        (`KismetSystemLibrary.K2_SetTimer` null "Fire" (/ 1.0 (`self.DPS`)) true)))))

(event `InputAxis|MoveUp`
  (params (AxisValue :type "Float (single-precision)"))
  ;[1 1 1] Movement
  (`self.AddMovementInput` (1.0 0.0 0.0) AxisValue))

(event `InputAxis|Aim Right`
  (params (AxisValue :type "Float (single-precision)"))
  ;[1 1 1] Rotation
  (goto _label))

(event `InputAction|Pause Game`
  (params (Key :type "Key Structure"))
  (bind _returnvalue (`GameplayStatics.GetPlayerController` 0))
  (bind _pause_menu_ref (`self.Pause Menu REF`))
  ;[1 1 1] Pause / Un Pause Game
  (:`Pressed`
    (`/Engine/EditorBlueprintResources/StandardMacros.IsValid` (`self.Pause Menu REF`)
      (:`Is Valid`
        _)
      (:`Is Not Valid`
        (bind _returnvalue_2 (`|CreateWidget` "/Game/PauseMenu/PauseMenuWidget.PauseMenuWidget_C"))
        (set `self.Pause Menu REF` _returnvalue_2)))
    (if (`GameplayStatics.IsGamePaused`)
      (`Widget.RemoveFromParent` _pause_menu_ref)
      (`GameplayStatics.SetGamePaused` false)
      (set `PlayerController.bShowMouseCursor` false _returnvalue)
      (`WidgetBlueprintLibrary.SetInputMode_GameOnly` _returnvalue)
      (else
        (`UserWidget.AddToViewport` _pause_menu_ref 0)
        (`GameplayStatics.SetGamePaused` true)
        (set `PlayerController.bShowMouseCursor` true _returnvalue)
        (`WidgetBlueprintLibrary.SetInputMode_GameAndUIEx` _returnvalue _pause_menu_ref "LockInFullscreen" false)))))

(fn `UserConstructionScript`)