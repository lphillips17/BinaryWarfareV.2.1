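; Sprite-based enemy that gets a random tint on spawn through a dynamic material instance.
; On overlapping an actor it sends a 5-damage message, runs the health drop and destroys itself.
; The drop traces down to the ground and occasionally spawns a HealthPowerup at a random reachable point nearby, using a random Select with mostly empty options.
; A polarity switch event only stores its Switch value.
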(event `self.ReceiveBeginPlay`
  (bind _returnvalue (`PrimitiveComponent.CreateDynamicMaterialInstance` (`self.Green_No__1_Sprite_0`) 0 null "None"))
  (`MaterialInstanceDynamic.SetVectorParameterValue` _returnvalue "Color" (make `LinearColor` (`KismetMathLibrary.RandomFloat`) (`KismetMathLibrary.RandomFloat`) (`KismetMathLibrary.RandomFloat`) 1.0)))

(event `self.ReceiveActorBeginOverlap`
  (params (OtherActor :type "Actor Object Reference"))
  (message `/Game/Blueprints/Damageable.Take Damage` OtherActor 5.0)
  (`self.Health Drop`)
  (`self.K2_DestroyActor`))

(event `Polarity Switch 1`
  (params (Switch :type Boolean :default true))
  ;[1 1 1] Polarity Switch
  (set `self.Switch` Switch))

(event `Health Drop`
  (bind _returnvalue (`self.K2_GetActorLocation`))
  ;[1 1 1] Health Drop System
  (bind _outhit (`KismetSystemLibrary.LineTraceSingle` _returnvalue (- _returnvalue (0.0 0.0 200.0)) "TraceTypeQuery1" false (`|MakeArray` (`GameplayStatics.GetPlayerCharacter` 0) :!type "Actor Object Reference")))
  (`|SpawnActorFromClass` (select `int` (`KismetMathLibrary.RandomInteger` 10) :`0` "/Game/Blueprints/HealthPowerup.HealthPowerup_C" :`1` null :`2` null :`3` null :`4` null :`5` null :`6` null :!type "Actor Class Reference") (`KismetMathLibrary.MakeTransform` (`NavigationSystemV1.K2_GetRandomReachablePointInRadius` (`.Location` (`GameplayStatics.BreakHitResult` _outhit)) 100.0 null null)) "AdjustIfPossibleButDontSpawnIfColliding" "OverrideRootScale" null null))

(fn `UserConstructionScript`)