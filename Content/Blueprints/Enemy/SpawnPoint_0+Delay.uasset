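; Enemy spawn point actor that keeps adding Enemy_AI_0 pawns at random positions inside its Bound box.
; Tick runs through a 10-second Delay, which throttles the world count of Enemy_AI_0 actors into a periodic check.
; While fewer than ten exist, it waits a further Time delay, then spawns one running the Enemy_AI_Behaviour behavior tree.
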(event `self.ReceiveTick`
  (params (DeltaSeconds :type "Float (single-precision)"))
  (bind _bound (`self.Bound`))
  (`KismetSystemLibrary.Delay` 10.0)
  (bind _outactors (`GameplayStatics.GetAllActorsOfClass` "/Game/Blueprints/Enemy/Enemy_AI_0.Enemy_AI_0_C"))
  (if (< (`KismetArrayLibrary.Array_Length` _outactors) 10)
    (`KismetSystemLibrary.Delay` (`self.Time`))
    (`AIBlueprintHelperLibrary.SpawnAIFromClass` "/Game/Blueprints/Enemy/Enemy_AI_0.Enemy_AI_0_C" "/Game/Blueprints/Enemy/Enemy_AI_Behaviour.Enemy_AI_Behaviour" (`KismetMathLibrary.RandomPointInBoundingBox` (`SceneComponent.K2_GetComponentLocation` _bound) (`BoxComponent.GetScaledBoxExtent` _bound)) (struct) false null)))

(fn `UserConstructionScript`)