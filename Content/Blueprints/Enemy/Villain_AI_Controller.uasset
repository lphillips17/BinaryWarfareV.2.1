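; AI controller for villain enemies that starts their behavior tree with the player as the target.
; Possess caches the controlled pawn, then BeginPlay runs Enemy_AI_Behaviour and writes player pawn 0 and the cached pawn into the blackboard's enemy and self-actor keys.
; Both keys are set only once, and a failed tree start just prints a debug string.
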(event `self.ReceivePossess`
  (params (PossessedPawn :type "Pawn Object Reference"))
  (set `self.Self Actor` PossessedPawn))

(event `self.ReceiveBeginPlay`
  (bind _returnvalue (`self.RunBehaviorTree` "/Game/Blueprints/Enemy/Enemy_AI_Behaviour.Enemy_AI_Behaviour"))
  (if _returnvalue
    (`BlackboardComponent.SetValueAsObject` (`AIBlueprintHelperLibrary.GetBlackboard` null) (`self.Enemy Key`) (`GameplayStatics.GetPlayerPawn` 0))
    (`BlackboardComponent.SetValueAsObject` (`AIBlueprintHelperLibrary.GetBlackboard` null) (`self.Self Actor Key`) (`self.Self Actor`))
    (else
      (`KismetSystemLibrary.PrintString` "RunBehaviourTreeFalse"))))

(fn `UserConstructionScript`)