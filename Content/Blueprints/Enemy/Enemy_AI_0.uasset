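; Enemy AI 0 is a sprite enemy actor that tints itself a random color at BeginPlay through a dynamic material instance.
; On overlap it sends a fixed-damage TakeDamageMessage to the other actor, then destroys itself if its Switch flag is true.
; The PolaritySwitch event sets and prints that flag, then runs the same destroy check, so switching it on removes the enemy immediately.
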(event `self.ReceiveBeginPlay`
  (bind _returnvalue (`PrimitiveComponent.CreateDynamicMaterialInstance` (`self.Green_No__1_Sprite_0`) 0 null "None"))
  (`MaterialInstanceDynamic.SetVectorParameterValue` _returnvalue "Color" (make `LinearColor` (`KismetMathLibrary.RandomFloat`) (`KismetMathLibrary.RandomFloat`) (`KismetMathLibrary.RandomFloat`) 1.0)))

(event `self.ReceiveActorBeginOverlap`
  (params (OtherActor :type "Actor Object Reference"))
  (message `/Game/Blueprints/Damageable.Take Damage` OtherActor 5.0)
  (if (stale `Polarity Switch` _output_get) :!label _label
    (`self.K2_DestroyActor`)))

(event `Polarity Switch`
  (params (Switch :type Boolean :default true))
  ;[1 1 1] Polarity Switch
  (bind _output_get (set `self.Switch` Switch))
  (`KismetSystemLibrary.PrintString` (`KismetStringLibrary.Conv_BoolToString` _output_get))
  (goto _label))

(fn `UserConstructionScript`)